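; Player marine pawn that moves on fixed world axes, aims by mouse motion and creates its HUD on BeginPlay.
; Each tick, when mouse velocity exceeds a dead zone, control yaw interpolates toward the direction of that motion, independent of cursor position.
; Fire input toggles the rifle particle effect and firing sound, with an end sound on release; no projectile or damage logic is present.
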(event `self.ReceiveTick`
  (params (DeltaSeconds :type "Float (single-precision)"))
  (`self.Update Player Aim`))

(event `self.ReceiveBeginPlay`
  (bind _returnvalue (`|CreateWidget` "/Game/UMG/WB_HUD_01.WB_HUD_01_C" null self))
  (`UserWidget.AddToViewport` _returnvalue 0))

(event `InputAction|Fire`
  (params (Key :type "Key Structure"))
  (:`Pressed`
    (`self.StartFire`))
  (:`Released`
    (`self.StopFire`)))

(event `InputAxis|MoveForwardBack`
  (params (AxisValue :type "Float (single-precision)"))
  (`self.AddMovementInput` (1.0 0.0 0.0) AxisValue))

(event `InputAxis|MoveLeftRight`
  (params (AxisValue :type "Float (single-precision)"))
  (`self.AddMovementInput` (0.0 -1.0 0.0) AxisValue))

(fn `GetMouseVelocity`
  (returns (`ReturnValue ` :type "Vector2D Structure"))
  (bind (_deltax _deltay) (`PlayerController.GetInputMouseDelta` (`GameplayStatics.GetPlayerController` 0)))
  (return (/ (`KismetMathLibrary.MakeVector2D` _deltax _deltay) (`GameplayStatics.GetWorldDeltaSeconds`))))

(fn `Is Mouse Above Dead Zone`
  (returns (ReturnValue :type Boolean))
  (return (> (`KismetMathLibrary.VSize2D` (`self.GetMouseVelocity`)) (`self.Mouse Dead Zone`))))

(fn `StartFire`
  (`ActorComponent.Activate` (`self.P_AssaultRifle_MF`) false)
  (bind _returnvalue (`GameplayStatics.SpawnSound2D` "/Game/Sounds/Weapon_AssaultRifle/Stereo/SC_Fire_01.SC_Fire_01" 1.0 1.0 0.0 null))
  (set `self.Audio_Fire_01` _returnvalue)
  (return))

(fn `StopFire`
  (`ActorComponent.Deactivate` (`self.P_AssaultRifle_MF`))
  (`AudioComponent.Stop` (`self.Audio_Fire_01`))
  (`GameplayStatics.SpawnSound2D` "/Game/Sounds/Weapon_AssaultRifle/Stereo/SC_EndFire_01.SC_EndFire_01" 1.0 1.0 0.0 null))

(fn `Update Player Aim`
  (locals (DeltaTimeMultiply :type "Float (double-precision)" :default 7.0))
  (bind _returnvalue (`GameplayStatics.GetPlayerController` 0))
  (bind (_x _y) (`KismetMathLibrary.BreakVector2D` (`self.GetMouseVelocity`)))
  (if (`self.Is Mouse Above Dead Zone`)
    (`Controller.SetControlRotation` _returnvalue (`KismetMathLibrary.RInterpTo` (`Controller.GetControlRotation` _returnvalue) (`KismetMathLibrary.MakeRotator` 0.0 0.0 (`KismetMathLibrary.DegAtan2` _x _y)) (`GameplayStatics.GetWorldDeltaSeconds`) (`local.DeltaTimeMultiply`)))))

(fn `UserConstructionScript`)