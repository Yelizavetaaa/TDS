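; Player character pawn that moves along fixed world axes and turns to face the direction of mouse movement.
; Forward/back and left/right axis inputs add movement on world X and Y, independent of facing.
; Each tick, when mouse velocity (delta over frame time) exceeds a dead zone, its atan2 angle becomes the target yaw.
; Control rotation interpolates toward that yaw, with pitch and roll targeted at zero.
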(event `self.ReceiveTick`
  (params (DeltaSeconds :type "Float (single-precision)"))
  (`self.Update Player Rotation`))

(event `InputAxis|MoveForwardBack`
  (params (AxisValue :type "Float (single-precision)"))
  (`self.AddMovementInput` (1.0 0.0 0.0) AxisValue))

(event `InputAxis|MoveLeftRight`
  (params (AxisValue :type "Float (single-precision)"))
  (`self.AddMovementInput` (0.0 -1.0 0.0) AxisValue))

(fn `GetMouseVelocity`
  (returns (`ReturnValue ` :type "Vector2D Structure"))
  (bind (_deltax _deltay) (`PlayerController.GetInputMouseDelta` (`GameplayStatics.GetPlayerController` 0)))
  (return (/ (`KismetMathLibrary.MakeVector2D` _deltax _deltay) (`GameplayStatics.GetWorldDeltaSeconds`))))

(fn `IsMouseAboveDeadZone`
  (returns (ReturnValue :type Boolean))
  (return (> (`KismetMathLibrary.VSize2D` (`self.GetMouseVelocity`)) (`self.Mouse Dead Zone`))))

(fn `Update Player Rotation`
  (locals (DeltaTimeMultiply :type "Float (double-precision)" :default 7.0))
  (bind _returnvalue (`GameplayStatics.GetPlayerController` 0))
  (bind (_x _y) (`KismetMathLibrary.BreakVector2D` (`self.GetMouseVelocity`)))
  (if (`self.IsMouseAboveDeadZone`)
    (`Controller.SetControlRotation` _returnvalue (`KismetMathLibrary.RInterpTo` (`Controller.GetControlRotation` _returnvalue) (`KismetMathLibrary.MakeRotator` 0.0 0.0 (`KismetMathLibrary.DegAtan2` _x _y)) (`GameplayStatics.GetWorldDeltaSeconds`) (`local.DeltaTimeMultiply`)))))

(fn `UserConstructionScript`)